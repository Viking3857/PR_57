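; Light actor Blueprint that blinks three point lights in staggered sequences when play begins.
; On BeginPlay, three Sequence branches start after different delays, each looping through a DoN node to toggle its light's visibility on and off with its own count and duration variables.
; The construction script sets the initial visibility of all three lights from IsEnableLight.
; The remaining functions are empty stubs, apart from one that returns the light components.
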(event `self.ReceiveBeginPlay`
  (`|ExecutionSequence`
    (:`then_0`
      (`KismetSystemLibrary.Delay` 0.1)
      (`/Engine/EditorBlueprintResources/StandardMacros.Do N` (`self.amount 1`) :!label _label
        (:`Exit`
          (`KismetSystemLibrary.Delay` (`self.Duration1`))
          (`SceneComponent.SetVisibility` (`self.PointLight`) true false)
          (`KismetSystemLibrary.Delay` (`self.Duration1`))
          (`SceneComponent.SetVisibility` (`self.PointLight`) false false)
          (goto _label))))
    (:`then_1`
      (`KismetSystemLibrary.Delay` 2.0)
      (`/Engine/EditorBlueprintResources/StandardMacros.Do N` (`self.amount 2`) :!label _label_2
        (:`Exit`
          (`KismetSystemLibrary.Delay` (`self.Duration2`))
          (`SceneComponent.SetVisibility` (`self.PointLight1`) true true)
          (`KismetSystemLibrary.Delay` (`self.Duration2`))
          (`SceneComponent.SetVisibility` (`self.PointLight1`) false true)
          (goto _label_2))))
    (:`then_2`
      (`KismetSystemLibrary.Delay` 6.0)
      (`/Engine/EditorBlueprintResources/StandardMacros.Do N` (`self.amount 3`) :!label _label_3
        (:`Exit`
          (`KismetSystemLibrary.Delay` (`self.Duration3`))
          (`SceneComponent.SetVisibility` (`self.PointLight2`) true true)
          (`KismetSystemLibrary.Delay` (`self.Duration3`))
          (`SceneComponent.SetVisibility` (`self.PointLight2`) false true)
          (goto _label_3))))))

(fn `Cube-1`)

(fn `Cube-1-1`)

(fn `NewFunction`
  (returns (PointLight1 :type "PointLightComponent Object Reference") (PointLight2 :type "PointLightComponent Object Reference") (PointLight :type "PointLightComponent Object Reference"))
  (return (`self.PointLight1`) (`self.PointLight2`) (`self.PointLight`)))

(fn `NewFunction_0`)

(fn `Sphere1`)

(fn `UserConstructionScript`
  (`SceneComponent.SetVisibility` (`self.PointLight`) (`self.Is Enable Light`) false)
  (`SceneComponent.SetVisibility` (`self.PointLight1`) (`self.Is Enable Light`) false)
  (`SceneComponent.SetVisibility` (`self.PointLight2`) (`self.Is Enable Light`) false))